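; BP_Doc is a test Blueprint that downloads a public Google Sheet as CSV at BeginPlay and prints the results on screen.
; It fires two requests to the same URL, one printing the raw response string.
; The other validates the download with backup fallback, fills the BranTestPing0 struct array, and prints one row's Username and Password.
; Unwired leftover nodes reference a DocTestPing food-bin array.
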(event Custom|CustomEvent_0
  (params (CallbackInfo :type Runtime%20Data%20Table%20Callback%20Info%20Structure))
  (bind _brantestping_0 (Variables|Default|GetBranTestPing_0))
  (bind _output (Utilities|Array|Get(acopy) _brantestping_0 9))
  (bind (_membervar_0 _username _password) (Utilities|Struct|BreakBPing _output))
  (bind _outcsvinfo (Class|RuntimeDataTableObject|ValidateGoogleSheetsDownloadandLoadBackupifNeeded CallbackInfo))
  (bind _successful (Class|RuntimeDataTableObject|UpdateArrayfromCsvInfo _brantestping_0 _outcsvinfo))
  (if _successful
    (Development|PrintString "Well The stuff should be in an array" true true "(R=1.000000,G=0.000000,B=0.000000,A=1.000000)" 6e+01)
    (Development|PrintText (Utilities|Text|FormatText "{Username}, {Password}" _username _password) true true "(R=0.000000,G=0.043803,B=0.354167,A=1.000000)" 6e+01)
    (Development|PrintString _password true true "(R=0.000000,G=0.000000,B=0.000000,A=1.000000)" 6e+01)))

(event Custom|CustomEvent_1
  (params (CallbackInfo :type Runtime%20Data%20Table%20Callback%20Info%20Structure))
  (Development|PrintString (.responseasstring CallbackInfo) true true "(R=1.000000,G=1.000000,B=1.000000,A=1.000000)" 6e+01))

(event EventBeginPlay
  (bind _binturl (Variables|Default|GetBintUrl))
  (Class|RuntimeDataTableObject|BuildGoogleSheetDownloadLinkandGetasCsv :CallOnComplete (delegate Custom|CustomEvent_0) :InSheetURL _binturl :bSheetIsPublic true)
  (Class|RuntimeDataTableObject|BuildGoogleSheetDownloadLinkandGetasCsv :CallOnComplete (delegate Custom|CustomEvent_1) :InSheetURL _binturl :bSheetIsPublic true))

(fn ConstructionScript)